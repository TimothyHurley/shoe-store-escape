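; Player controller for mouse drawing that turns a freehand stroke into a straight line.
; Creates a W_Drawable widget and, while left mouse is held, appends DPI-scaled cursor positions to its LinePoints on Tick.
; On release, it estimates stroke length from alternating segments doubled, then scales the start-to-last-point vector to that length.
; The result sets the widget's EndingPosition and flags IsBestFitLine; GetLineDirection classifies quadrants but is not called here.
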(event EventBeginPlay
  (bind _returnvalue (UserInterface|CreateWidget "/Game/Blueprints/Widgets/W_Drawable.W_Drawable_C" self))
  (UserInterface|Viewport|AddtoViewport _returnvalue -1)
  (bind _output_get (Variables|Default|SetDrawableRef _returnvalue))
  (Input|SetInputModeGameandUI self _output_get "DoNotLock" false)
  (Variables|Default|SetbShowMouseCursor true))

(event EventTick
  (params (DeltaSeconds :type Float%20%28single-precision%29))
  (bind _self self)
  (bind _self_2 self)
  (bind _drawableref (Variables|Default|GetDrawableRef))
  (bind (_locationx _locationy) (Class|WidgetLayoutLibrary|GetMousePositionScaledbyDPI _self_2))
  (bind (_locationx_2 _locationy_2) (Class|WidgetLayoutLibrary|GetMousePositionScaledbyDPI _self))
  (bind _linepoints (Variables|/Game/Blueprints/Widgets/W_Drawable.W_Drawable_C|GetLinePoints _drawableref))
  (if (Variables|Default|GetIsLeftMouseButtonDown?)
    (if (> (Utilities|Array|Length (Variables|/Game/Blueprints/Widgets/W_Drawable.W_Drawable_C|GetLinePoints (Variables|Default|GetDrawableRef))) 0)
      (if (not (Math|Vector|Equal(Vector) (Utilities|Array|Get(acopy) _linepoints (Utilities|Array|LastIndex _linepoints)) (Math|Vector2D|MakeVector2D _locationx_2 _locationy_2) 0.1))
        (Utilities|Array|Add (Variables|/Game/Blueprints/Widgets/W_Drawable.W_Drawable_C|GetLinePoints (Variables|Default|GetDrawableRef)) (Math|Vector2D|MakeVector2D _locationx _locationy) :!label _label))
      (else
        (goto _label)))))

(event Input|MouseEvents|LeftMouseButton
  (params (Key :type Key%20Structure :default "None"))
  (bind _self self)
  (bind _self_2 self)
  (bind _drawableref (Variables|Default|GetDrawableRef))
  (bind _drawableref_2 (Variables|Default|GetDrawableRef))
  (bind (_locationx _locationy) (Class|WidgetLayoutLibrary|GetMousePositionScaledbyDPI _self_2))
  (bind (_locationx_2 _locationy_2) (Class|WidgetLayoutLibrary|GetMousePositionScaledbyDPI _self))
  (bind _linepoints (Variables|/Game/Blueprints/Widgets/W_Drawable.W_Drawable_C|GetLinePoints _drawableref))
  (bind _returnvalue (Utilities|Array|LastIndex _linepoints))
  (bind _output (Utilities|Array|Get(acopy) _linepoints _returnvalue))
  (:Pressed
    (Variables|Default|SetStartingX _locationx_2)
    (Variables|Default|SetStartingY _locationy_2)
    (Variables|/Game/Blueprints/Widgets/W_Drawable.W_Drawable_C|SetStartingPosition _drawableref_2 (Math|Vector2D|MakeVector2D (Variables|Default|GetStartingX) (Variables|Default|GetStartingY)))
    (Default|ResetVariables _drawableref_2)
    (CallFunction|ResetVariables)
    (Variables|Default|SetIsLeftMouseButtonDown? true))
  (:Released
    (Variables|Default|SetEndingX _locationx)
    (Variables|Default|SetEndingY _locationy)
    (Variables|Default|SetIsLeftMouseButtonDown? false)
    (Variables|Default|SetIsSecondPoint? false)
    (for _array_element (Variables|/Game/Blueprints/Widgets/W_Drawable.W_Drawable_C|GetLinePoints (Variables|Default|GetDrawableRef))
      (if (Variables|Default|GetIsSecondPoint?)
        (Variables|Default|SetPaintLength (+ (Variables|Default|GetPaintLength) (CallFunction|CalculatePaintLength (.x _array_element) (.y _array_element))))
        (Variables|Default|SetIsSecondPoint? false)
        (else
          (Variables|Default|SetTempStartingX (.x _array_element))
          (Variables|Default|SetTempStartingY (.y _array_element))
          (Variables|Default|SetIsSecondPoint? true))))
    (Variables|Default|SetPaintLength (* (Variables|Default|GetPaintLength) 2.0))
    (CallFunction|SetRiseandRun (.x _output) (.y _output))
    (Variables|Default|SetLineLength (CallFunction|CalculateLineLength))
    (CallFunction|UpdateRiseandRun)
    (CallFunction|UpdateEndingPosition)
    (Variables|/Game/Blueprints/Widgets/W_Drawable.W_Drawable_C|SetIsBestFitLine? _drawableref true)))

(fn ConstructionScript)

(fn ResetVariables
  (Variables|Default|SetRise 0.0)
  (Variables|Default|SetRun 0.0)
  (Variables|Default|SetPaintLength 0.0)
  (Variables|Default|SetLineLength 0.0)
  (Variables|Default|SetIsFacingNorthWest? false)
  (Variables|Default|SetIsFacingNorthEast? false)
  (Variables|Default|SetIsFacingSouthWest? false)
  (Variables|Default|SetIsFacingSouthEast? false)
  (return))

(fn CalculatePaintLength
  (params (X :type Float%20%28single-precision%29) (Y :type Float%20%28single-precision%29))
  (bind _tempstartingx (Variables|Default|GetTempStartingX))
  (bind _tempstartingy (Variables|Default|GetTempStartingY))
  (bind _returnvalue (- X _tempstartingx))
  (bind _returnvalue_2 (- Y _tempstartingy))
  (return (Math|Float|Sqrt (+ (* _returnvalue _returnvalue) (* _returnvalue_2 _returnvalue_2)))))

(fn CalculateLineLength
  (return (Math|Float|Sqrt (+ (* (Variables|Default|GetRise) (Variables|Default|GetRise)) (* (Variables|Default|GetRun) (Variables|Default|GetRun))))))

(fn CalculateLegLength
  (return (+ (- (Variables|Default|GetPaintLength) (Variables|Default|GetLineLength)) (Variables|Default|GetLineLength))))

(fn CalculateLengthMultiplier
  (return (/ (Variables|Default|GetPaintLength) (Variables|Default|GetLineLength))))

(fn SetRiseandRun
  (params (X :type Float%20%28single-precision%29) (Y :type Float%20%28single-precision%29))
  (Variables|Default|SetRun (- X (Variables|Default|GetStartingX)))
  (Variables|Default|SetRise (- Y (Variables|Default|GetStartingY))))

(fn GetLineDirection
  (bind _drawableref (Variables|Default|GetDrawableRef))
  (bind _startingposition (Variables|/Game/Blueprints/Widgets/W_Drawable.W_Drawable_C|GetStartingPosition _drawableref))
  (bind _endingposition (Variables|/Game/Blueprints/Widgets/W_Drawable.W_Drawable_C|GetEndingPosition _drawableref))
  (LocalVariables|SetLocalStartingX (.x _startingposition))
  (LocalVariables|SetLocalStartingY (.y _startingposition))
  (LocalVariables|SetLocalEndingX (.x _endingposition))
  (LocalVariables|SetLocalEndingY (.y _endingposition))
  (if (and (< (LocalVariables|GetLocalEndingX) (LocalVariables|GetLocalStartingX)) (<= (LocalVariables|GetLocalEndingY) (LocalVariables|GetLocalStartingY)))
    (Variables|Default|SetIsFacingNorthWest? true)
    (elif (and (<= (LocalVariables|GetLocalStartingX) (LocalVariables|GetLocalEndingX)) (< (LocalVariables|GetLocalEndingY) (LocalVariables|GetLocalStartingY)))
      (Variables|Default|SetIsFacingNorthEast? true)
      (elif (and (<= (LocalVariables|GetLocalEndingX) (LocalVariables|GetLocalStartingX)) (< (LocalVariables|GetLocalStartingY) (LocalVariables|GetLocalEndingY)))
        (Variables|Default|SetIsFacingSouthWest? true)
        (elif (and (< (LocalVariables|GetLocalStartingX) (LocalVariables|GetLocalEndingX)) (<= (LocalVariables|GetLocalStartingY) (LocalVariables|GetLocalEndingY)))
          (Variables|Default|SetIsFacingSouthEast? true)))))
  (return))

(fn UpdateRiseandRun
  (bind _lengthmultiplier (CallFunction|CalculateLengthMultiplier))
  (Variables|Default|SetRise (* (Variables|Default|GetRise) _lengthmultiplier))
  (Variables|Default|SetRun (* (Variables|Default|GetRun) _lengthmultiplier))
  (return))

(fn UpdateEndingPosition
  (bind _drawableref (Variables|Default|GetDrawableRef))
  (bind _startingposition (Variables|/Game/Blueprints/Widgets/W_Drawable.W_Drawable_C|GetStartingPosition _drawableref))
  (LocalVariables|SetLocalStartingX (.x _startingposition))
  (LocalVariables|SetLocalStartingY (.y _startingposition))
  (LocalVariables|SetLocalEndingPosition (Variables|/Game/Blueprints/Widgets/W_Drawable.W_Drawable_C|GetEndingPosition _drawableref))
  (LocalVariables|SetLocalEndingPosition (Math|Vector2D|MakeVector2D (+ (LocalVariables|GetLocalStartingX) (Variables|Default|GetRun)) (+ (LocalVariables|GetLocalStartingY) (Variables|Default|GetRise))))
  (Variables|/Game/Blueprints/Widgets/W_Drawable.W_Drawable_C|SetEndingPosition (Variables|Default|GetDrawableRef) (LocalVariables|GetLocalEndingPosition))
  (return))